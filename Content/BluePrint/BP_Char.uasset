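; BP_Char is a player Character Blueprint with axis-driven look and movement plus a double jump.
; Look axes feed controller yaw and inverted pitch, and move axes push along the actor's right and forward vectors.
; Jump uses LaunchCharacter at the movement component's jump velocity with Z override, gated by a DoN of two that resets on landing.
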(event `InputAxis|Look_Right`
  (params (AxisValue :type "Float (single-precision)"))
  ;[1 1 1] Looking
  (`self.AddControllerYawInput` AxisValue))

(event `InputAxis|Look_Up`
  (params (AxisValue :type "Float (single-precision)"))
  ;[1 1 1] Looking
  (`self.AddControllerPitchInput` (* AxisValue -1.0)))

(event `InputAxis|Move_Right`
  (params (AxisValue :type "Float (single-precision)"))
  ;[1 1 1] Movement
  (`self.AddMovementInput` (`self.GetActorRightVector`) AxisValue))

(event `InputAxis|Move_Forward`
  (params (AxisValue :type "Float (single-precision)"))
  ;[1 1 1] Movement
  (`self.AddMovementInput` (`self.GetActorForwardVector`) AxisValue))

(event `InputAction|Jump`
  (params (Key :type "Key Structure"))
  ;[1 1 1] Actions
  (:`Pressed`
    (`/Engine/EditorBlueprintResources/StandardMacros.Do N` 2 :!label _label
      (:`Exit`
        (`self.LaunchCharacter` (`KismetMathLibrary.MakeVector` 0.0 0.0 (`CharacterMovementComponent.JumpZVelocity` (`self.CharacterMovement`))) false true)))))

(event `self.OnLanded`
  (params (Hit :type "HitResult Structure (by ref)"))
  ;[1 1 1] Actions
  (goto _label :!via `Reset`))

(fn `UserConstructionScript`)